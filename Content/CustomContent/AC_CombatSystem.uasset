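; Combat component for a Character owner that plays a chain of sword attack montages as a combo.
; BeginPlay caches the owner's mesh, and TriggerAttack plays the montage at the current combo index, then advances the index, wrapping after the last.
; Montage notify begin and end toggle the CanAttack flag to form a window for chaining the next attack.
; Montage completion re-enables attacking and resets the combo to the first attack.
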(event Custom|TriggerAttack
  (Variables|Default|GetbCanAttack
    (:then
      (Variables|Default|SetbCanAttack false)
      (bind _notifyname (Animation|Montage|PlayMontage (Variables|Default|GetCharacterMesh) (Utilities|Array|Get(acopy) (Variables|SystemParameters|GetAttackAnimsSword) (Variables|Default|GetAttackIndexCurrent)))
        (:then
          (Variables|Default|SetAttackIndexCurrent (Math|Integer|SelectInt (+ (Variables|Default|GetAttackIndexCurrent) 1) 0 (< (Variables|Default|GetAttackIndexCurrent) (Utilities|Array|LastIndex (Variables|SystemParameters|GetAttackAnimsSword))))))
        (:OnCompleted
          (Variables|Default|SetbCanAttack true)
          (Variables|Default|SetAttackIndexCurrent 0))
        (:OnNotifyBegin
          (switch name _notifyname
            (:ComboInputWindow
              (Variables|Default|SetbCanAttack true))))
        (:OnNotifyEnd
          (switch name _notifyname
            (:ComboInputWindow
              (Variables|Default|SetbCanAttack false))))))
    (:else)))

(event EventBeginPlay
  (bind _ascharacter (Utilities|Casting|CastToCharacter (Components|GetOwner)))
  (Variables|Default|SetCharacterMesh (Variables|/Script/Engine.Character|GetMesh _ascharacter)))