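; BP_PurifyZone is a zone actor that drives a purification effect in the MPC_Corruption material parameter collection when the player character enters it.
; On BeginPlay it writes its radius and world location to the collection as the purify radius and origin.
; A sphere overlap by BP_FilRougeCharacter calls ActivatePurification, which plays a timeline that animates PurifyStrength.
; Because the parameters are collection-wide, each instance overwrites the same values.
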(event OnComponentBeginOverlap(Sphere)
  (params (OverlappedComponent :type Primitive%20Component%20Object%20Reference) (OtherActor :type Actor%20Object%20Reference) (OtherComp :type Primitive%20Component%20Object%20Reference) (OtherBodyIndex :type Integer) (bFromSweep :type Boolean) (SweepResult :type Hit%20Result%20Structure%20%28by%20ref%29))
  (Utilities|Casting|CastToBP_FilRougeCharacter OtherActor)
  (CallFunction|ActivatePurification))

(event Custom|ActivatePurification
  (bind _strength (Timeline|T_PurifyFade Play)
    (:Update
      (Rendering|Material|SetScalarParameterValue "/Game/CustomContent/Materials/Corruption/MPC_Corruption.MPC_Corruption" "PurifyStrength" _strength :!class /Script/Engine.KismetMaterialLibrary))))

(event EventBeginPlay
  (Rendering|Material|SetScalarParameterValue "/Game/CustomContent/Materials/Corruption/MPC_Corruption.MPC_Corruption" "PurifyRadius" (Variables|Default|GetPurifyRadiusBP) :!class /Script/Engine.KismetMaterialLibrary)
  (Rendering|Material|SetVectorParameterValue "/Game/CustomContent/Materials/Corruption/MPC_Corruption.MPC_Corruption" "PurifyOrigin" (Math|Conversions|ToLinearColor(Vector) (Transformation|GetActorLocation)) :!class /Script/Engine.KismetMaterialLibrary))

(event Collision|EventActorBeginOverlap
  (params (OtherActor :type Actor%20Object%20Reference)))

(event EventTick
  (params (DeltaSeconds :type Float%20%28single-precision%29)))

(fn ConstructionScript)