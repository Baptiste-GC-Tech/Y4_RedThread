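; BP_Sword is an interactable sword pickup that attaches to the player's hand.
; On player interaction it sets the AsSword flag and attaches to the HandGrip_R socket on the player 0 character's mesh, snapping position and rotation while keeping world scale.
; It then disables the interaction collision and limits the static mesh to physics-only collision.
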(event EventBeginPlay
  (|CallParentFunction) ; This node is disabled and will not be called.\nDrag off pins to build functionality.
)

(event Collision|EventActorBeginOverlap
  (params (OtherActor :type Actor%20Object%20Reference)))

(event EventTick
  (params (DeltaSeconds :type Float%20%28single-precision%29))
  (|CallParentFunction DeltaSeconds) ; This node is disabled and will not be called.\nDrag off pins to build functionality.
)

(event EventOnPlayerInteract
  (params (InteractingPlayerController :type Player%20Controller%20Object%20Reference))
  (Variables|Default|SetbAsSword true)
  (Transformation|AttachComponentToComponent (Variables|/Script/Engine.Character|GetMesh (Game|GetPlayerCharacter 0)) "HandGrip_R" "SnapToTarget" "SnapToTarget" "KeepWorld" true)
  (Collision|SetCollisionEnabled (Variables|Default|GetInteractableCollision) "NoCollision")
  (Collision|SetCollisionEnabled (Variables|Default|GetStaticMesh) "PhysicsOnly"))

(fn ConstructionScript
  (|CallParentFunction))