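; BP_BasicSolvable is a simple solvable actor that shows its solved state through a point light.
; On BeginPlay it binds ChangeVisuals to the solve-state-updated dispatcher, which turns the light green when solved and red otherwise.
; UpdateSolveState only calls the parent, so this Blueprint adds just the visual feedback and no solve logic of its own.
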(event Custom|ChangeVisuals
  (params (SolvableUpdated :type B%20Pabs%20GEN%20Solvable%20Object%20Reference) (isSolved :type Boolean))
  (if isSolved
    (Variables|Var|SetNewLinearColor "(R=0.000000,G=1.000000,B=0.000000,A=1.000000)")
    (else
      (Variables|Var|SetNewLinearColor "(R=1.000000,G=0.000000,B=0.000000,A=1.000000)")))
  (Rendering|Components|Light|SetLightColor (Variables|Default|GetPointLight) (Variables|Var|GetNewLinearColor) true))

(event EventBeginPlay
  (|CallParentFunction)
  (EventDispatchers|BindEventtoEDonSolveStateUpd (delegate Custom|ChangeVisuals)))

(event Collision|EventActorBeginOverlap
  (params (OtherActor :type Actor%20Object%20Reference))
  (|CallParentFunction OtherActor) ; This node is disabled and will not be called.\nDrag off pins to build functionality.
)

(event EventTick
  (params (DeltaSeconds :type Float%20%28single-precision%29))
  (|CallParentFunction DeltaSeconds))

(event EventUpdateSolveState
  (|CallParentFunction))

(fn ConstructionScript
  (|CallParentFunction))