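; Solvable door that slides its mesh between closed and open positions when its solve state changes.
; BeginPlay binds OpenOrCloseDoor to the solve-state dispatcher, which moves DoorMesh over TransitionTime via MoveComponentTo.
; The construction script scales the mesh and caches the closed position from door height.
; The open position is offset from the mesh's current location, raised by its height minus a small lip; the moving flag does not block retriggering.
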(event Custom|OpenOrCloseDoor
  (params (SolvableUpdated :type B%20Pabs%20GEN%20Solvable%20Object%20Reference) (isSolved :type Boolean))
  (bind _doormesh (Variables|Default|GetDoorMesh))
  (if (Variables|Var|DoorAnim|GetisDoorMeshMoving)
    _
    (else
      _))
  (Variables|Var|DoorAnim|SetisDoorMeshMoving true)
  (Components|MoveComponentTo _doormesh (CallFunction|DetermineAnimPos isSolved) (Variables|/Script/Engine.SceneComponent|GetRelativeRotation _doormesh) false false (Variables|Var|DoorAnim|GetTransitionTime) false)
  (Variables|Var|DoorAnim|SetisDoorMeshMoving false))

(event EventBeginPlay
  (|CallParentFunction)
  (EventDispatchers|UnbindEventfromEDonSolveStateUpd (delegate Custom|OpenOrCloseDoor))
  (EventDispatchers|BindEventtoEDonSolveStateUpd (delegate Custom|OpenOrCloseDoor)))

(event EventUpdateSolveState)

(event EventDestroyed)

(fn ConstructionScript
  (bind _doormesh (Variables|Default|GetDoorMesh))
  (bind _doorscalez (Variables|Var|Visuals|GetDoorScaleZ))
  (bind _returnvalue (* _doorscalez 5e+01))
  (bind _relativelocation (Variables|/Script/Engine.SceneComponent|GetRelativeLocation _doormesh))
  (bind (_x _y) (Math|Vector|BreakVector _relativelocation))
  (bind _returnvalue_2 (Math|Vector|MakeVector _x _y _returnvalue))
  (|CallParentFunction)
  (Utilities|FlowControl|Sequence
    (:then_0
      (Transformation|SetRelativeScale3D _doormesh (Math|Vector|MakeVector (.X (Math|Vector|BreakVector (Variables|/Script/Engine.SceneComponent|GetRelativeScale3D _doormesh))) (Variables|Var|Visuals|GetDoorScaleY) (Variables|Var|Visuals|GetDoorScaleZ))))
    (:then_1
      (Transformation|SetRelativeLocation _doormesh _returnvalue_2 false false)
      (Variables|Var|Door|SetCachedClosedPos _returnvalue_2))))

(fn DetermineOpenPos
  (bind _doormesh (Variables|Default|GetDoorMesh))
  (bind _relativelocation (Variables|/Script/Engine.SceneComponent|GetRelativeLocation _doormesh))
  (bind (_x _y) (Math|Vector|BreakVector _relativelocation))
  (return (- (+ _relativelocation (Math|Vector|MakeVector _x _y (* (Variables|Var|Visuals|GetDoorScaleZ) 1e+02))) "0.000000,0.000000,10.000000")))

(fn DetermineAnimPos
  (params (isSolved :type Boolean))
  (if isSolved
    (if (Variables|Default|GetisSolved)
      (return (CallFunction|DetermineOpenPos))
      (else
        (return (Variables|Var|Door|GetOpenPosition))))
    (else
      (return (Variables|Var|Door|GetCachedClosedPos)))))