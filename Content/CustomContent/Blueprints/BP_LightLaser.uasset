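; BP_LightLaser is a spline-based actor that forms a laser shape from deformed cylinder meshes.
; The construction script adds one Z-forward spline mesh per spline segment, fitted to that segment's local endpoints and tangents.
; An UpdateLightLaser event replaces the spline's points in local space but does not itself rebuild or move the meshes.
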(event Custom|UpdateLightLaser
  (params (NewSplinePoints :type Array%20of%20Vectors))
  (Spline|SetSplinePoints (Variables|Default|GetSpline) NewSplinePoints "Local" true))

(event EventBeginPlay)

(event EventTick
  (params (DeltaSeconds :type Float%20%28single-precision%29)))

(fn ConstructionScript
  (bind _spline (Variables|Default|GetSpline))
  ;[0.15 0.15 0.15 0.5] Go through all Spline Segments (with indexes)
  (for _index (range 0 (- (Class|SplineComponent|GetNumberOfSplineSegments _spline) 1))
    (bind _returnvalue (AddComponent|AddSplineMeshComponent false)) ; This node has a Details menu with extra data.\nUses the default Cylinder, with "Forward Axis" at Z because of that.
    (SplineMesh|SetStartandEnd _returnvalue (.Location (Spline|GetLocationandTangentatSplinePoint _spline _index "Local")) (.Tangent (Spline|GetLocationandTangentatSplinePoint _spline _index "Local")) (.Location (Spline|GetLocationandTangentatSplinePoint _spline (+ _index 1) "Local")) (.Tangent (Spline|GetLocationandTangentatSplinePoint _spline (+ _index 1) "Local")) true :!class /Script/Engine.SplineMeshComponent)))