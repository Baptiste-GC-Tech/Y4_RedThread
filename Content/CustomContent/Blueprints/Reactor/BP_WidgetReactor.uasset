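; Interactable reactor actor that opens and closes the WBP_PuzzleEau water puzzle widget when OnInteractionNOARGS fires.
; The first interaction creates the widget and adds it to the viewport; later ones toggle its visibility through an open flag.
; Opening shows the mouse cursor and switches to UI-only input focused on the widget, while closing hides the cursor and restores game-only input.
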(event EventBeginPlay)

(event Collision|EventActorBeginOverlap
  (params (OtherActor :type Actor%20Object%20Reference)))

(event EventTick
  (params (DeltaSeconds :type Float%20%28single-precision%29)))

(event EventOnInteractionNOARGS
  (params (InteractableCaller :type B%20Pabs%20GEN%20Interactable%20Object%20Reference))
  (bind _returnvalue (Game|GetPlayerController 0))
  (Development|PrintString "Hello")
  (if (Variables|Var|GetWBPHasBeenInitialized)
    (if (Variables|Var|GetWBPIsOpen)
      (Variables|Var|SetWBPIsOpen false)
      (Widget|SetVisibility (Variables|Default|GetWBPToOpen) "Collapsed")
      (Variables|/Script/Engine.PlayerController|SetbShowMouseCursor _returnvalue false)
      (Input|SetInputModeGameOnly _returnvalue false)
      (Development|PrintString "Jouer")
      (else
        (Variables|Var|SetWBPIsOpen true)
        (Widget|SetVisibility (Variables|Default|GetWBPToOpen) "Visible")
        (Variables|/Script/Engine.PlayerController|SetbShowMouseCursor _returnvalue true :!label _label)
        (Input|SetInputModeUIOnly _returnvalue (Variables|Default|GetWBPToOpen) "DoNotLock" false)
        (Development|PrintString "Interagir")))
    (else
      (Variables|Var|SetWBPHasBeenInitialized true)
      (Variables|Var|SetWBPIsOpen true)
      (bind _returnvalue_2 (Game|ConstructObjectfromClass "/Game/CustomContent/Blueprints/Widgets/Puzzle_Eau/WBP_PuzzleEau.WBP_PuzzleEau_C"))
      (bind _output_get (Variables|Default|SetWBPToOpen _returnvalue_2))
      (UserInterface|Viewport|AddtoViewport _output_get 0)
      (goto _label))))

(fn ConstructionScript)