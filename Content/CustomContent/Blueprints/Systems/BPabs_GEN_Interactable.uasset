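; Abstract-style base Blueprint for interactable objects that can drive puzzle Solvables and other reactor Actors.
; A collision component shows and hides an interaction prompt widget on overlap, with debug prints; the prompt text is updatable.
; On player interaction, it asks each listed Solvable to update its solve state, then triggers non-puzzle reactors, passing itself, for feedback or effects like opening doors.
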(event OnComponentBeginOverlap(InteractableCollision)
  (params (OverlappedComponent :type Primitive%20Component%20Object%20Reference) (OtherActor :type Actor%20Object%20Reference) (OtherComp :type Primitive%20Component%20Object%20Reference) (OtherBodyIndex :type Integer) (bFromSweep :type Boolean) (SweepResult :type Hit%20Result%20Structure%20%28by%20ref%29))
  ;[0.15 0.15 0.15 0.5] UI management
  (Development|PrintString "Overlap +" true false "(R=0.059198,G=0.109774,B=1.000000,A=1.000000)")
  (Rendering|SetVisibility (Variables|Default|GetInteractionWidget) true false))

(event OnComponentEndOverlap(InteractableCollision)
  (params (OverlappedComponent :type Primitive%20Component%20Object%20Reference) (OtherActor :type Actor%20Object%20Reference) (OtherComp :type Primitive%20Component%20Object%20Reference) (OtherBodyIndex :type Integer))
  ;[0.15 0.15 0.15 0.5] UI management
  (Development|PrintString "Overlap -" true false "(R=0.059198,G=0.109774,B=1.000000,A=1.000000)")
  (Rendering|SetVisibility (Variables|Default|GetInteractionWidget) false false))

(event EventBeginPlay
  ;[0.15 0.15 0.15 0.5] UI management
  (Rendering|SetVisibility (Variables|Default|GetInteractionWidget) false false))

(event EventOnPlayerInteract
  (params (InteractingPlayerController :type Player%20Controller%20Object%20Reference))
  (CallFunction|UpdateAllSolvables) ; Attempts to solve any Solvables listed.\nThis will probably do nothing on Solvables with conditions.
  (CallFunction|TriggerAllReactorsNOARGS) ; Triggers any Actors that aren't puzzles.\nCould be useful for feedback or opening a door.
)

(fn ConstructionScript)

(fn TriggerAllReactorsNOARGS
  (for _array_element (Variables|Var|GetTriggeredReactors_NOARGS)
    (Default|OnInteractionNOARGS _array_element self)))

(fn UpdateAllSolvables
  (for _array_element (Variables|Var|GetUpdatedSolvables)
    (Default|UpdateSolveState _array_element)))

(fn UpdateInteractionText
  (params (NewString :type String))
  (Default|SetInteractionText (.AsWBP%20Interact%20Prompt (Utilities|Casting|CastToWBP_InteractPrompt (UserInterface|GetWidget (Variables|Default|GetInteractionWidget)))) NewString))