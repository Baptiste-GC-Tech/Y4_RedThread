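; Interactable laser emitter that fires a bouncing beam to solve light receivers when the player interacts with it.
; Each interaction clears LaserSpline to its first point, then DoOneRaycast traces, notifies receivers and appends spline points for the beam path.
; PrepareNextRaycast mirrors the ray off the hit normal, looping until a miss, an absorbing receiver or the bounce cap.
; HasRayBeenAbsorbed reads inverted: false means absorbed.
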(event EventBeginPlay
  (|CallParentFunction))

(event EventTick
  (params (DeltaSeconds :type Float%20%28single-precision%29))
  (|CallParentFunction DeltaSeconds))

(event EventOnPlayerInteract
  (params (InteractingPlayerController :type Player%20Controller%20Object%20Reference))
  (bind _returnvalue (Transformation|GetActorLocation))
  (bind _returnvalue_2 (Transformation|GetActorTransform))
  (bind _initialraycastlocaloffset (Variables|Var|Raycasting|GetInitialRaycastLocalOffset))
  (bind _laserspline (Variables|Default|GetLaserSpline))
  (bind _returnvalue_3 (Math|Transform|TransformDirection _returnvalue_2 _initialraycastlocaloffset))
  (bind _returnvalue_4 (+ _returnvalue _returnvalue_3))
  (|CallParentFunction InteractingPlayerController)
  ;[0.01266 0.132 0.15 0.5] Spline full reset
  (bind _output_get (Variables|Var|Spline|SetcurSplineSegmentCount (Class|SplineComponent|GetNumberOfSplineSegments _laserspline)))
  (for _index (range 1 _output_get) ; Never removes the first spline point.\nThis conserves the spline's very start.
    (Spline|RemoveSplinePoint _laserspline 1 false) ; Removes the point following the spline's start.\nIndexes are updated in this operation (all after : decrem'd) ¬.¬
  )
  (Spline|UpdateSpline _laserspline)
  (Development|PrintString "Cleaned spline !" true true "(R=1.000000,G=0.311457,B=0.000000,A=1.000000)" 1e+01)
  (Variables|Var|Raycasting|SetSecurityCounter 0)
  (Variables|Var|Raycasting|SethasRayBeenAbsorbed true)
  ;[0.15 0.15 0.15 0.5] Prepares the first raycast
  (Variables|Var|Raycasting|SetCurRaycastStartingPoint _returnvalue_4)
  (Variables|Var|Raycasting|SetCurRaycastEndingPoint (+ _returnvalue_4 (* (Variables|Var|Raycasting|GetraycastLength) (Math|Vector|GetForwardVector (Transformation|GetActorRotation)))))
  ;[0.15 0.15 0.15 0.5] Do...
  (bind (_impactpoint _impactnormal _rayforwardvector) (CallFunction|DoOneRaycast))
  (if (Variables|Var|Raycasting|GethasLastRayHit)
    (CallFunction|PrepareNextRaycast _impactpoint _impactnormal _rayforwardvector)
    ;[0.15 0.15 0.15 0.5] ...While
    (while (Math|Boolean|ANDBoolean (Variables|Var|Raycasting|GethasRayBeenAbsorbed) (Variables|Var|Raycasting|GethasLastRayHit) (< (Variables|Var|Raycasting|GetSecurityCounter) (Variables|Var|Raycasting|GetMaxSubsequentRaycasts)))
      (bind (_impactpoint_2 _impactnormal_2 _rayforwardvector_2) (CallFunction|DoOneRaycast))
      (CallFunction|PrepareNextRaycast _impactpoint_2 _impactnormal_2 _rayforwardvector_2)
      (Math|Integer|IncrementInt (Variables|Var|Raycasting|GetSecurityCounter)))))

(fn ConstructionScript
  (|CallParentFunction))

(fn DoOneRaycast
  (bind _curraycaststartingpoint (Variables|Var|Raycasting|GetCurRaycastStartingPoint))
  (bind _curraycastendingpoint (Variables|Var|Raycasting|GetCurRaycastEndingPoint))
  (bind _returnvalue (- _curraycastendingpoint _curraycaststartingpoint))
  (bind _returnvalue_2 (Math|Vector|Normalize _returnvalue))
  (bind (_outhits _returnvalue_3) (Collision|MultiLineTraceByChannel (Variables|Var|Raycasting|GetCurRaycastStartingPoint) (Variables|Var|Raycasting|GetCurRaycastEndingPoint) "TraceTypeQuery3" false 0 "ForDuration" true "(R=1.000000,G=0.000000,B=0.000000,A=1.000000)" "(R=0.000000,G=1.000000,B=0.000000,A=1.000000)" (Variables|Var|Raycasting|GetDebug%20Draw%20Time))) ; Could be a single Raycast\nMulti is meant for piercing rays, which this is not at the time or writing this
  (for _array_element _outhits
    (Development|PrintString "Entered DoOneRaycast Foreach !" true true "(R=1.000000,G=0.000000,B=0.021578,A=1.000000)" 1e+01)
    ;[0 0 0 0.5] Content of the ForEach's loop
    ;;[0.15 0.15 0.15 0.5] Tests if the line trace collided with a BPI_SolvableByLight
    (if (and (.bBlockingHit (Collision|BreakHitResult _array_element)) (Utilities|DoesObjectImplementInterface (.HitActor (Collision|BreakHitResult _array_element)) "/Game/CustomContent/Blueprints/Systems/SpecificSolvables/LightPuzzle/BPI_SolvableByLight.BPI_SolvableByLight_C"))
      (Development|PrintString "Solved a light recier" true true "(R=0.046875,G=1.000000,B=0.047206,A=1.000000)" 1e+01)
      ;;[0.15 0.09132 0.01768 0.5] Ray absorption support
      (if (.bSuccess (Utilities|Casting|CastToBP_LightReceiver (.HitActor (Collision|BreakHitResult _array_element))))
        (if (Variables|/Game/CustomContent/Blueprints/Solvables/BP_LightReceiver.BP_LightReceiver_C|GetdoesAbsorbLight (.AsBP%20Light%20Receiver (Utilities|Casting|CastToBP_LightReceiver (.HitActor (Collision|BreakHitResult _array_element)))))
          (Variables|Var|Raycasting|SethasRayBeenAbsorbed false))
        (Default|OnLightSolve (.AsBP%20Light%20Receiver (Utilities|Casting|CastToBP_LightReceiver (.HitActor (Collision|BreakHitResult _array_element)))) self)
        ;;[0.554 0.1389 0.6146 0.5] Feeds the spline with point to display the laser later
        (if (.bBlockingHit (Collision|BreakHitResult _array_element)) :!label _label
          (LocalVariables|SetSplinePosThisRaycast (.ImpactPoint (Collision|BreakHitResult _array_element)))
          (else
            (LocalVariables|SetSplinePosThisRaycast (Variables|Var|Raycasting|GetCurRaycastEndingPoint))))
        (Spline|AddSplinePoint (Variables|Default|GetLaserSpline) (LocalVariables|GetSplinePosThisRaycast) "World" true) ; Updates spline for each added points, but whatever
        (Development|PrintString (Utilities|String|Append "+ Spline Point at " (Utilities|String|ToString(Vector) (LocalVariables|GetSplinePosThisRaycast))) true true "(R=1.000000,G=0.329541,B=0.000000,A=1.000000)" 1e+01))
      (else
        (goto _label))))
  (Variables|Var|Raycasting|SethasLastRayHit _returnvalue_3)
  (Development|PrintString (Utilities|String|Append "Im Pt : " (Utilities|String|ToString(Vector) (+ (.ImpactPoint (Collision|BreakHitResult _array_element)) (* (Math|Float|MakeLiteralFloat 0.01) (.ImpactNormal (Collision|BreakHitResult _array_element))))) "  |  Im Norm : " (Utilities|String|ToString(Vector) (.ImpactNormal (Collision|BreakHitResult _array_element))) "  |  Ray Forw Vect : " (Utilities|String|ToString(Vector) _returnvalue_2)))
  (return (+ (.ImpactPoint (Collision|BreakHitResult _array_element)) (* (Math|Float|MakeLiteralFloat 0.01) (.ImpactNormal (Collision|BreakHitResult _array_element)))) (.ImpactNormal (Collision|BreakHitResult _array_element)) _returnvalue_2))

(fn PrepareNextRaycast
  (params (LastImpactPoint :type Vector) (LastImpactNormal :type Vector) (LastRayForwardVector :type Vector))
  (bind _output_get (Variables|Var|Raycasting|SetCurRaycastStartingPoint LastImpactPoint))
  (bind _output_get_2 (Variables|Var|Raycasting|SetCurRaycastEndingPoint (+ LastImpactPoint (* (Math|Vector|MirrorVectorbyNormal LastRayForwardVector LastImpactNormal) (Variables|Var|Raycasting|GetraycastLength))))))