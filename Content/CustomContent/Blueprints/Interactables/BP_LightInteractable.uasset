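; BP_LightInteractable is an interactable whose point light switches color each time the player interacts with it.
; On interaction it tries to update its linked puzzle Solvables, then triggers non-puzzle reactor Actors through inherited-style helper calls.
; A FlipFlop then toggles IsOn, which selects a teal light color when on and orange when off.
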(event EventBeginPlay
  (|CallParentFunction) ; This node is disabled and will not be called.\nDrag off pins to build functionality.
)

(event Collision|EventActorBeginOverlap
  (params (OtherActor :type Actor%20Object%20Reference))
  (|CallParentFunction OtherActor) ; This node is disabled and will not be called.\nDrag off pins to build functionality.
)

(event EventTick
  (params (DeltaSeconds :type Float%20%28single-precision%29))
  (|CallParentFunction DeltaSeconds) ; This node is disabled and will not be called.\nDrag off pins to build functionality.
)

(event EventOnPlayerInteract
  (params (InteractingPlayerController :type Player%20Controller%20Object%20Reference))
  (CallFunction|UpdateAllSolvables) ; Attempts to solve any Solvables listed.\nThis will probably do nothing on Solvables with conditions.
  (CallFunction|TriggerAllReactorsNOARGS) ; Triggers any Actors that aren't puzzles.\nCould be useful for feedback or opening a door.
  (Utilities|FlowControl|FlipFlop
    (:A
      (Variables|Var|SetisOn true))
    (:B
      (Variables|Var|SetisOn false)))
  (if (Variables|Var|GetisOn)
    (Variables|Var|SetNew%20Light%20Color "(R=0.000000,G=0.700000,B=0.600000,A=1.000000)")
    (else
      (Variables|Var|SetNew%20Light%20Color "(R=1.000000,G=0.300544,B=0.000000,A=1.000000)")))
  (Rendering|Components|Light|SetLightColor (Variables|Default|GetPointLight) (Variables|Var|GetNew%20Light%20Color) true))

(fn ConstructionScript
  (|CallParentFunction))