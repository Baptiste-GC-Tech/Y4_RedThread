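; BP_MiasmaOrb is a puzzle target orb that registers hits from BP_Arrow overlaps on its sphere.
; The first hit in an attempt sets a hit flag and, if a puzzle manager reference is valid, reports the orb to it, hides the orb and disables collision.
; ResetOrb clears the flag and restores visibility and query-only collision.
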(event OnComponentBeginOverlap(Sphere)
  (params (OverlappedComponent :type Primitive%20Component%20Object%20Reference) (OtherActor :type Actor%20Object%20Reference) (OtherComp :type Primitive%20Component%20Object%20Reference) (OtherBodyIndex :type Integer) (bFromSweep :type Boolean) (SweepResult :type Hit%20Result%20Structure%20%28by%20ref%29))
  (bind _puzzlemanagerref (Variables|Default|GetPuzzleManagerRef))
  (Utilities|Casting|CastToBP_Arrow OtherActor)
  (Variables|Default|GetbHitThisAttempt
    (:then)
    (:else
      (Variables|Default|SetbHitThisAttempt true)
      (Utilities|IsValid _puzzlemanagerref
        (:Is%20Valid
          (Default|RegisterOrbHit _puzzlemanagerref self)
          (Rendering|SetVisibility (Variables|Default|GetOrb) false false)
          (Collision|SetCollisionEnabled (Variables|Default|GetSphere) "NoCollision"))))))

(event EventBeginPlay)

(event Collision|EventActorBeginOverlap
  (params (OtherActor :type Actor%20Object%20Reference)))

(event EventTick
  (params (DeltaSeconds :type Float%20%28single-precision%29)))

(fn ConstructionScript)

(fn ResetOrb
  (Variables|Default|SetbHitThisAttempt false)
  (Rendering|SetVisibility (Variables|Default|GetOrb) true false)
  (Collision|SetCollisionEnabled (Variables|Default|GetSphere) "QueryOnly"))