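; Actor component that gives its owning Character bow aiming, drawing and arrow firing.
; Aiming switches rotation to follow controller yaw and attaches a spawned BP_Arrow to a mesh socket, while updating the state of the BP_Bow found in the level.
; A looping timer accumulates draw time, which becomes normalized strength when the arrow fires along the camera's forward vector.
; After a short delay, a new arrow spawns if still aiming.
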(event Custom|AimStart
  (bind _charref (Variables|Default|GetCharRef))
  (bind _charactermovement (Variables|/Script/Engine.Character|GetCharacterMovement _charref))
  (Variables|Default|SetIsAiming true)
  (Variables|/Script/Engine.CharacterMovementComponent|SetbOrientRotationToMovement _charactermovement false)
  (Variables|/Script/Engine.CharacterMovementComponent|SetbUseControllerDesiredRotation _charactermovement true)
  (Variables|/Script/Engine.CharacterMovementComponent|SetRotationRate _charactermovement (Variables|Default|GetAimRotationRate))
  (Variables|/Game/CustomContent/Blueprints/Combat/Weapons/BP_Bow.BP_Bow_C|SetBowState (Variables|Default|GetRefBow) "NewEnumerator1")
  (CallFunction|SpawnActor))

(event Custom|AimEnd
  (bind _charref (Variables|Default|GetCharRef))
  (bind _charactermovement (Variables|/Script/Engine.Character|GetCharacterMovement _charref))
  (Variables|Default|SetIsAiming false)
  (CallFunction|DrawEnd)
  (Variables|/Script/Engine.CharacterMovementComponent|SetbOrientRotationToMovement _charactermovement true)
  (Variables|/Script/Engine.CharacterMovementComponent|SetbUseControllerDesiredRotation _charactermovement false)
  (Variables|/Script/Engine.CharacterMovementComponent|SetRotationRate _charactermovement (Variables|Default|GetInitialRotationRate))
  (Variables|/Game/CustomContent/Blueprints/Combat/Weapons/BP_Bow.BP_Bow_C|SetBowState (Variables|Default|GetRefBow) "NewEnumerator0")
  (CallFunction|DestroyActor))

(event Custom|FireArrowBegin
  (if (Variables|Default|GetIsDrawingBow)
    (Variables|Default|SetIsFiringArrow true)
    (CallFunction|FireAimArrow)
    (CallFunction|DrawEnd)
    (Utilities|FlowControl|Delay 1.0)
    (CallFunction|FireArrowEnd)))

(event Custom|DrawBegin
  (Utilities|CanDrawBow
    (:Yes
      (Variables|Default|SetIsDrawingBow true)
      (bind _returnvalue (Utilities|Time|SetTimerbyEvent (delegate Custom|IncrementTime) (Variables|Default|GetDrawIncrementTime) true))
      (Variables|Default|SetDrawTimer _returnvalue)
      (Variables|/Game/CustomContent/Blueprints/Combat/Weapons/BP_Bow.BP_Bow_C|SetBowState (Variables|Default|GetRefBow) "NewEnumerator2"))))

(event Custom|DrawEnd
  (Variables|Default|SetIsDrawingBow false)
  (Variables|Default|SetDrawTime 0.0)
  (Utilities|Time|ClearandInvalidateTimerbyHandle (Variables|Default|GetDrawTimer))
  (Variables|/Game/CustomContent/Blueprints/Combat/Weapons/BP_Bow.BP_Bow_C|SetBowState (Variables|Default|GetRefBow) "NewEnumerator0"))

(event Custom|IncrementTime
  (bind _output_get (Variables|Default|SetDrawTime (+ (Variables|Default|GetDrawTime) (Variables|Default|GetDrawIncrementTime))))
  (Development|PrintString (Utilities|String|ToString(Float) _output_get)))

(event Custom|FireArrowEnd
  (Variables|Default|SetIsFiringArrow false)
  (if (Variables|Default|GetIsAiming)
    (CallFunction|AimStart)))

(event EventBeginPlay
  (bind _ascharacter (Utilities|Casting|CastToCharacter (Components|GetOwner)))
  (Variables|Default|SetCharRef _ascharacter)
  (Variables|Default|SetInitialRotationRate (Variables|/Script/Engine.CharacterMovementComponent|GetRotationRate (Variables|/Script/Engine.Character|GetCharacterMovement (Variables|Default|GetCharRef))))
  (bind _returnvalue (Actor|GetActorOfClass "/Game/CustomContent/Blueprints/Combat/Weapons/BP_Bow.BP_Bow_C"))
  (Variables|Default|SetRefBow _returnvalue))

(event EventTick
  (params (DeltaSeconds :type Float%20%28single-precision%29)))

(fn SpawnActor
  (bind _returnvalue (Game|SpawnActorfromClass "/Game/CustomContent/Blueprints/Combat/Weapons/BP_Arrow.BP_Arrow_C" (Math|Transform|MakeTransform "0, 0, 0" "0, 0, 0" "1.000000,1.000000,1.000000") "Undefined" "MultiplyWithRoot" 0 0))
  (bind _output_get (Variables|Default|SetArrowRef _returnvalue))
  (Transformation|AttachComponentToComponent _output_get (Variables|/Script/Engine.Character|GetMesh (Variables|Default|GetCharRef)) (Variables|Default|GetArrowSocketName) "SnapToTarget" "SnapToTarget" "SnapToTarget" true))

(fn DestroyActor
  (bind _arrowref (Variables|Default|GetArrowRef)
    (:then
      (Actor|DestroyActor _arrowref))
    (:else)))

(fn FireAimArrow
  (bind _arrowref (Variables|Default|GetArrowRef)
    (:then
      (Transformation|DetachFromActor _arrowref "KeepWorld" "KeepWorld" "KeepWorld")
      (Default|Fire _arrowref (Math|Vector|GetForwardVector (Actor|GetComponentbyClass (Variables|Default|GetCharRef) "/Script/Engine.CameraComponent")) (Math|Float|Clamp(Float) (Math|Float|NormalizetoRange (Variables|Default|GetDrawTime) 0.0 (Variables|/Game/CustomContent/Blueprints/Combat/Weapons/BP_Bow.BP_Bow_C|GetMaxDrawTime (Variables|Default|GetRefBow))))))
    (:else)))