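; AC_HitStop is an actor component that applies a hit-stop effect to its owning Character by changing that character's time dilation.
; On BeginPlay it casts and caches the owner as a Character.
; BeginHitStop sets the character's CustomTimeDilation to the given value and starts a timer for the given duration.
; EndHitStop restores the dilation to normal, affecting only that character rather than global time.
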(event Custom|BeginHitStop
  (params (Duration :type Float%20%28double-precision%29) (TimeDilation :type Float%20%28double-precision%29))
  (Variables|/Script/Engine.Actor|SetCustomTimeDilation (Variables|Default|GetCharacterActor) TimeDilation)
  (Utilities|Time|SetTimerbyEvent (EventDispatchers|CreateEvent :!event Custom|EndHitStop) Duration))

(event Custom|EndHitStop
  (Variables|/Script/Engine.Actor|SetCustomTimeDilation (Variables|Default|GetCharacterActor) 1.0))

(event EventBeginPlay
  (bind _ascharacter (Utilities|Casting|CastToCharacter (Components|GetOwner)))
  (Variables|Default|SetCharacterActor _ascharacter))