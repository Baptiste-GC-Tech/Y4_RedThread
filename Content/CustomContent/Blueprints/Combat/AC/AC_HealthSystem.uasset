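; Health component for Characters that tracks damage, drives a health bar and handles death.
; BeginPlay binds damage, spawns screen-space bars for all but player 0 and gets or adds an AC_HitStop component.
; Death disables damage and pawn collision and stops enemy AI, then pauses with a death screen for the player or destroys others on a montage notify.
; Heal clamps to current rather than max health, so it cannot raise health.
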(event Custom|ProcessDamage
  (params (DamageAmount :type Float%20%28double-precision%29))
  (bind _returnvalue (Game|GetPlayerController 0))
  (bind _characteractor (Variables|Default|GetCharacterActor))
  (Variables|Default|SetCurrentHealthPoints (Math|Float|Max(Float) (- (Variables|Default|GetCurrentHealthPoints) DamageAmount) 0.0))
  (CallFunction|RefreshBar)
  (if (<= (Variables|Default|GetCurrentHealthPoints) 0.0)
    (bind _asaic_enemy_base (Utilities|Casting|CastToAIC_EnemyBase (AI|GetAIController (Components|GetOwner)))
      (:then
        (AI|Logic|StopLogic (Variables|/Script/AIModule.AIController|GetBrainComponent _asaic_enemy_base) "Died"))
      (:CastFailed
        _))
    (Variables|/Script/Engine.Actor|SetbCanBeDamaged _characteractor false)
    (Collision|SetCollisionResponsetoChannel (Variables|/Script/Engine.Character|GetCapsuleComponent _characteractor) "ECC_Pawn" "ECR_Ignore")
    (if (== (Variables|Default|GetCharacterActor) (Game|GetPlayerCharacter 0))
      (bind _returnvalue_2 (UserInterface|CreateWidget "/Game/CustomContent/UI/WBP_Death.WBP_Death_C" (Game|GetPlayerController 0)))
      (UserInterface|Viewport|AddtoViewport _returnvalue_2 0)
      (Input|SetInputModeUIOnly _returnvalue _returnvalue_2 "DoNotLock" false)
      (Variables|/Script/Engine.PlayerController|SetbShowMouseCursor _returnvalue true)
      (Game|SetGamePaused true)
      (else
        (Animation|Montage|PlayMontage (Variables|/Script/Engine.Character|GetMesh _characteractor) (Variables|Default|GetDeathMontagePlay)
          (:OnNotifyBegin
            (Actor|DestroyActor (Variables|Default|GetCharacterActor))
            (Widget|SetVisibility (Variables|Default|GetHealthBar) "Hidden")))))))

(event Custom|OnTakeAnyDamage_Event
  (params (DamagedActor :type Actor%20Object%20Reference) (Damage :type Float%20%28single-precision%29) (DamageType :type Damage%20Type%20Object%20Reference) (InstigatedBy :type Controller%20Object%20Reference) (DamageCauser :type Actor%20Object%20Reference))
  (CallFunction|ProcessDamage Damage))

(event Custom|SpawnHealthBar
  (bind _characteractor (Variables|Default|GetCharacterActor))
  (bind _returnvalue (UserInterface|CreateWidget "/Game/CustomContent/UI/WBP_HealthBar.WBP_HealthBar_C"))
  (Variables|Default|SetHealthBar _returnvalue)
  (bind _returnvalue_2 (Game|AddComponentbyClass _characteractor "/Script/UMG.WidgetComponent" false (Math|Transform|MakeTransform (Math|Vector|MakeVector 0.0 0.0 (+ (Variables|/Script/Engine.CapsuleComponent|GetCapsuleHalfHeight (Variables|/Script/Engine.Character|GetCapsuleComponent _characteractor)) (Variables|Default|GetHealthBarZ_Offset))) "0, 0, 0" "1.000000,1.000000,1.000000")))
  (Class|WidgetComponent|SetWidgetSpace _returnvalue_2 "Screen")
  (UserInterface|SetWidget _returnvalue_2 (Variables|Default|GetHealthBar))
  (Class|WidgetComponent|SetDrawSize _returnvalue_2 (Variables|Default|GetHealthBarSize)))

(event EventBeginPlay
  (bind _ascharacter (Utilities|Casting|CastToCharacter (Components|GetOwner)))
  (bind _output_get (Variables|Default|SetCharacterActor _ascharacter))
  (EventDispatchers|AssignOnTakeAnyDamage _output_get (delegate Custom|OnTakeAnyDamage_Event))
  (Variables|Default|SetCurrentHealthPoints (Variables|Default|GetMaxHealthPoints))
  (if (== (Variables|Default|GetCharacterActor) (Game|GetPlayerCharacter 0))
    _
    (else
      (CallFunction|SpawnHealthBar)))
  (Utilities|IsValid (Actor|GetComponentbyClass (Variables|Default|GetCharacterActor) "/Game/CustomContent/Blueprints/Combat/AC/AC_HitStop.AC_HitStop_C")
    (:Is%20Valid
      (Variables|Default|SetHitStopComp (Actor|GetComponentbyClass (Variables|Default|GetCharacterActor) "/Game/CustomContent/Blueprints/Combat/AC/AC_HitStop.AC_HitStop_C")))
    (:Is%20Not%20Valid
      (bind _returnvalue (Game|AddComponentbyClass (Variables|Default|GetCharacterActor) "/Game/CustomContent/Blueprints/Combat/AC/AC_HitStop.AC_HitStop_C"))
      (Variables|Default|SetHitStopComp _returnvalue))))

(fn InitHealthBar
  (params (NewHealthBar :type WBP%20Health%20Bar%20Object%20Reference))
  (Variables|Default|SetHealthBar NewHealthBar))

(fn RefreshBar
  (Default|SetFillLevel (Variables|Default|GetHealthBar) (/ (Variables|Default|GetCurrentHealthPoints) (Variables|Default|GetMaxHealthPoints))))

(fn Heal
  (params (Amount :type Float%20%28double-precision%29))
  (Variables|Default|SetCurrentHealthPoints (Math|Float|Clamp(Float) (+ (Variables|Default|GetCurrentHealthPoints) Amount) 0.0 (Variables|Default|GetCurrentHealthPoints)))
  (CallFunction|RefreshBar))