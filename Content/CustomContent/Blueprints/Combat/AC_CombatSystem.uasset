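; Combat component for a Character owner that plays sword combo montages on the ground and a single attack montage when falling.
; Montage notifies open and close the combo window, and completion or landing resets the combo.
; TriggerHit sphere-traces between mesh sockets using an attack profile's radius, object types and damage.
; A HitActors list, cleared as each attack starts, limits damage to once per actor per swing.
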(event Custom|TriggerAttack
  (if (AI|Components|NavMovement|IsFalling (Variables|/Script/Engine.Character|GetCharacterMovement (Variables|Default|GetCharacterActor)))
    (CallFunction|AirAttack)
    (else
      (CallFunction|GroundAttack))))

(event Custom|AirAttack
  (Variables|Default|GetCanAirAttack
    (:then
      (Variables|Default|SetCanAirAttack false)
      (Utilities|Array|Clear (Variables|Default|GetHitActors))
      (Animation|Montage|PlayMontage (Variables|Default|GetCharacterMesh) (Variables|SystemParameters|GetAirAttackAnim) 1.2
        (:OnBlendOut
          (Variables|Default|SetCanAirAttack true))))
    (:else)))

(event Custom|GroundAttack
  (Variables|Default|GetbCanAttack
    (:then
      (Variables|Default|SetbCanAttack false)
      (Utilities|Array|Clear (Variables|Default|GetHitActors))
      (bind _notifyname (Animation|Montage|PlayMontage (Variables|Default|GetCharacterMesh) (Utilities|Array|Get(acopy) (Variables|SystemParameters|GetAttackAnimsSword) (Variables|Default|GetAttackIndexCurrent)))
        (:then
          (Variables|Default|SetAttackIndexCurrent (Math|Integer|SelectInt (+ (Variables|Default|GetAttackIndexCurrent) 1) 0 (< (Variables|Default|GetAttackIndexCurrent) (Utilities|Array|LastIndex (Variables|SystemParameters|GetAttackAnimsSword))))))
        (:OnCompleted
          (Variables|Default|SetbCanAttack true)
          (Variables|Default|SetAttackIndexCurrent 0))
        (:OnNotifyBegin
          (switch name _notifyname
            (:ComboInputWindow
              (Variables|Default|SetbCanAttack true))))
        (:OnNotifyEnd
          (switch name _notifyname
            (:ComboInputWindow
              (Variables|Default|SetbCanAttack false))))))
    (:else)))

(event Custom|OnCharacterLanded
  (params (Hit :type Hit%20Result%20Structure%20%28by%20ref%29))
  (Variables|Default|SetCanAirAttack true)
  (Variables|Default|SetbCanAttack true)
  (Variables|Default|SetAttackIndexCurrent 0)
  (if (== (Animation|GetCurrentMontage (Variables|Default|GetCharacterActor) :!class /Script/Engine.Character) (Variables|SystemParameters|GetAirAttackAnim))
    (Animation|StopAnimMontage (Variables|Default|GetCharacterActor) 0)))

(event Custom|TriggerHit
  (params (AttackProfile :type F%20Attack%20Profile%20Structure))
  (bind _charactermesh (Variables|Default|GetCharacterMesh))
  (bind (_outhits _returnvalue) (Collision|MultiSphereTraceForObjects (Transformation|GetSocketLocation _charactermesh (.startsocket AttackProfile)) (Transformation|GetSocketLocation _charactermesh (.endsocket AttackProfile)) (.hitsphereradius AttackProfile) (.hitableobjecttypes AttackProfile) false 0 "ForDuration"))
  (CallFunction|ApplyDamagetoHitActors (.damageamount AttackProfile) _returnvalue _outhits))

(event EventBeginPlay
  (bind _ascharacter (Utilities|Casting|CastToCharacter (Components|GetOwner)))
  (Variables|Default|SetCharacterActor _ascharacter)
  (Variables|Default|SetCharacterMesh (Variables|/Script/Engine.Character|GetMesh _ascharacter))
  (EventDispatchers|AssignLandedDelegate (Variables|Default|GetCharacterActor) (EventDispatchers|CreateEvent :!event Custom|OnCharacterLanded)))

(fn ApplyDamagetoHitActors
  (params (Amount :type Float%20%28double-precision%29) (Hit :type Boolean) (Hits :type Array%20of%20Hit%20Result%20Structures))
  (if Hit
    (for _array_element Hits
      (LocalVariables|SetHitActor (.HitActor (Collision|BreakHitResult _array_element)))
      (if (not (Utilities|Array|ContainsItem (Variables|Default|GetHitActors) (LocalVariables|GetHitActor)))
        (Game|Damage|ApplyDamage (LocalVariables|GetHitActor) Amount 0 (Variables|Default|GetCharacterActor))
        (Utilities|Array|Add (Variables|Default|GetHitActors) (LocalVariables|GetHitActor))))))