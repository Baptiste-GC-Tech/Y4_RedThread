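; BP_Bow is an interactable bow weapon that the player can pick up, equip and stow.
; Interacting unequips the BP_Sword cached at BeginPlay if its AsSword flag is set, then attaches the bow to the left-hand socket and disables pickup and mesh collision.
; Equip and UnEquip toggle the AsBow flag and move the bow between the hand and clavicle sockets on player 0's mesh.
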(event Custom|Equip
  (Variables|Default|SetAsBow true)
  (Transformation|AttachComponentToComponent (Variables|/Script/Engine.Character|GetMesh (Game|GetPlayerCharacter 0)) "HandGrip_L" "SnapToTarget" "SnapToTarget" "KeepWorld" true))

(event Custom|UnEquip
  (Variables|Default|SetAsBow false)
  (Transformation|AttachComponentToComponent (Variables|/Script/Engine.Character|GetMesh (Game|GetPlayerCharacter 0)) "clavicle_l_Bow" "KeepRelative" "KeepRelative" "KeepRelative" true))

(event EventBeginPlay
  (|CallParentFunction)
  (bind _returnvalue (Actor|GetActorOfClass "/Game/CustomContent/Blueprints/Combat/Weapons/BP_Sword.BP_Sword_C"))
  (Variables|Default|SetSwordRef _returnvalue))

(event Collision|EventActorBeginOverlap
  (params (OtherActor :type Actor%20Object%20Reference)))

(event EventTick
  (params (DeltaSeconds :type Float%20%28single-precision%29))
  (|CallParentFunction DeltaSeconds) ; This node is disabled and will not be called.\nDrag off pins to build functionality.
)

(event EventOnPlayerInteract
  (params (InteractingPlayerController :type Player%20Controller%20Object%20Reference))
  (bind _swordref (Variables|Default|GetSwordRef))
  (if (Variables|/Game/CustomContent/Blueprints/Combat/Weapons/BP_Sword.BP_Sword_C|GetbAsSword _swordref)
    (Default|Unequip _swordref))
  (Variables|Default|SetAsBow true)
  (Transformation|AttachComponentToComponent (Variables|/Script/Engine.Character|GetMesh (Game|GetPlayerCharacter 0)) "HandGrip_L" "SnapToTarget" "SnapToTarget" "KeepWorld" true)
  (Collision|SetCollisionEnabled (Variables|Default|GetInteractableCollision) "NoCollision")
  (Collision|SetCollisionEnabled (Variables|Default|GetGreatEagleBow_Animated) "NoCollision"))

(fn ConstructionScript
  (|CallParentFunction))