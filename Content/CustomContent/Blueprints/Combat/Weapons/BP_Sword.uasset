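; BP_Sword is an interactable sword weapon that the player picks up, equips and stows.
; On interaction it unequips the bow found at BeginPlay if that is active, snaps to the player mesh's right-hand socket and disables its interaction and mesh collision.
; Equip and Unequip toggle the AsSword flag and reattach the sword between the hand socket and the right-thigh socket.
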(event Custom|Equip
  (Variables|Default|SetbAsSword true)
  (Transformation|AttachComponentToComponent (Variables|/Script/Engine.Character|GetMesh (Game|GetPlayerCharacter 0)) "HandGrip_R" "SnapToTarget" "SnapToTarget" "KeepWorld" true))

(event Custom|Unequip
  (Variables|Default|SetbAsSword false)
  (Transformation|AttachComponentToComponent (Variables|/Script/Engine.Character|GetMesh (Game|GetPlayerCharacter 0)) "thigh_r_Sword" "KeepRelative" "KeepRelative" "KeepRelative" true))

(event EventBeginPlay
  (|CallParentFunction)
  (bind _returnvalue (Actor|GetActorOfClass "/Game/CustomContent/Blueprints/Combat/Weapons/BP_Bow.BP_Bow_C"))
  (Variables|Default|SetBowRef _returnvalue))

(event Collision|EventActorBeginOverlap
  (params (OtherActor :type Actor%20Object%20Reference)))

(event EventTick
  (params (DeltaSeconds :type Float%20%28single-precision%29))
  (|CallParentFunction DeltaSeconds) ; This node is disabled and will not be called.\nDrag off pins to build functionality.
)

(event EventOnPlayerInteract
  (params (InteractingPlayerController :type Player%20Controller%20Object%20Reference))
  (bind _bowref (Variables|Default|GetBowRef))
  (if (Variables|/Game/CustomContent/Blueprints/Combat/Weapons/BP_Bow.BP_Bow_C|GetAsBow _bowref)
    (Default|UnEquip _bowref))
  (Variables|Default|SetbAsSword true)
  (Transformation|AttachComponentToComponent (Variables|/Script/Engine.Character|GetMesh (Game|GetPlayerCharacter 0)) "HandGrip_R" "SnapToTarget" "SnapToTarget" "KeepWorld" true)
  (Collision|SetCollisionEnabled (Variables|Default|GetInteractableCollision) "NoCollision")
  (Collision|SetCollisionEnabled (Variables|Default|GetStaticMesh) "NoCollision"))

(fn ConstructionScript
  (|CallParentFunction))