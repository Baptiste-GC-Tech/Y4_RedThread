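; Arrow projectile that stays inert until fired, then flies with a trail effect and damages golems.
; Fire adds a projectile movement component at runtime, scaling speed and gravity by shot strength, and enables collision.
; On overlap with anything but its instigator, it stops and attaches to the hit component.
; Golem hits scale damage by hitbox name, more for head and less for feet, then destroy the arrow after a short delay.
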(event OnComponentHit(CollisionBox)
  (params (HitComponent :type Primitive%20Component%20Object%20Reference) (OtherActor :type Actor%20Object%20Reference) (OtherComp :type Primitive%20Component%20Object%20Reference) (NormalImpulse :type Vector :default "0, 0, 0") (Hit :type Hit%20Result%20Structure%20%28by%20ref%29))
  (bind _asbp_golem (Utilities|Casting|CastToBP_Golem OtherActor))
  (switch string (Utilities|GetObjectName OtherComp)
    (:Default
      _)
    (:HitboxHead
      (Variables|Default|SetDamage (* (Variables|Default|GetDamage) 2.0)))
    (:Hibox_footR
      (Variables|Default|SetDamage (* (Variables|Default|GetDamage) 0.5) :!label _label))
    (:Hibox_footL
      (goto _label)))
  (Game|Damage|ApplyDamage _asbp_golem (Variables|Default|GetDamage) 0 0)
  (Utilities|FlowControl|Delay 0.5)
  (Actor|DestroyActor))

(event OnComponentBeginOverlap(CollisionBox)
  (params (OverlappedComponent :type Primitive%20Component%20Object%20Reference) (OtherActor :type Actor%20Object%20Reference) (OtherComp :type Primitive%20Component%20Object%20Reference) (OtherBodyIndex :type Integer) (bFromSweep :type Boolean) (SweepResult :type Hit%20Result%20Structure%20%28by%20ref%29))
  (if (!= OtherActor (Game|GetInstigator))
    (bind _projectilecomponent (Variables|Default|GetProjectileComponent)
      (:then
        (Components|DestroyComponent _projectilecomponent))
      (:else
        _))
    (Collision|SetCollisionEnabled (Variables|Default|GetCollisionBox) "NoCollision")
    (Transformation|AttachComponentToComponent (.HitComponent (Collision|BreakHitResult SweepResult)) "None" "KeepWorld" "KeepWorld" "KeepWorld" true)))

(event Custom|Fire
  (params (Direction :type Vector) (Strenght :type Float%20%28double-precision%29))
  (bind _returnvalue (AddComponent|AddProjectileMovementComponent))
  (Variables|Default|SetProjectileComponent _returnvalue)
  (Variables|/Script/Engine.MovementComponent|SetVelocity _returnvalue (* Direction (Math|Float|Lerp (Variables|Default|GetMinSpeed) (Variables|Default|GetMaxSpeed) Strenght)))
  (Variables|/Script/Engine.ProjectileMovementComponent|SetProjectileGravityScale _returnvalue (Math|Float|Lerp (Variables|Default|GetMaxGravity) (Variables|Default|GetMinGravity) Strenght))
  (Niagara|SpawnSystemAttached "/Game/CustomContent/Materials/NS_ArrowTrail.NS_ArrowTrail" (Variables|Default|GetTrailEffectLocation) "None" "0, 0, 0" "0, 0, 0" "KeepRelativeOffset" false)
  (Collision|SetCollisionEnabled (Variables|Default|GetCollisionBox) "QueryAndPhysics"))

(event EventBeginPlay
  (Collision|SetCollisionEnabled (Variables|Default|GetCollisionBox) "NoCollision"))

(event EventTick
  (params (DeltaSeconds :type Float%20%28single-precision%29)))

(fn ConstructionScript)